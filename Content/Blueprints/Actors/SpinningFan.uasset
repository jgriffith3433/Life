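; Spinning fan actor that rotates continuously around its yaw axis and can have its spin direction flipped.
; Each tick rotates the Scene component by the current speed scaled by delta time, then steps that speed toward positive or negative maximum, clamped at the limit.
; ReverseSpin toggles the direction flag, so the fan eases through zero into the opposite spin.
; The speed step is applied per frame without delta time, making reversal frame-rate dependent.
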(event EventBeginPlay
  (Variables|Default|SetSpinSpeed (Variables|Default|GetMaxSpinSpeed)))

(event EventTick
  (params (DeltaSeconds :type Float%20%28single-precision%29))
  (Utilities|FlowControl|Sequence
    (:then_0
      (Transformation|AddRelativeRotation (Variables|Default|GetScene) (Math|Rotator|MakeRotator 0.0 0.0 (* (Variables|Default|GetSpinSpeed) DeltaSeconds)) false false))
    (:then_1
      (if (Variables|Default|GetbSpinReversed)
        (Variables|Default|SetSpinSpeed (- (Variables|Default|GetSpinSpeed) (Variables|Default|GetSpeedChange)))
        (if (< (Variables|Default|GetSpinSpeed) (* -1 (Variables|Default|GetMaxSpinSpeed)))
          (Variables|Default|SetSpinSpeed (* -1 (Variables|Default|GetMaxSpinSpeed))))
        (else
          (Variables|Default|SetSpinSpeed (+ (Variables|Default|GetSpinSpeed) (Variables|Default|GetSpeedChange)))
          (if (> (Variables|Default|GetSpinSpeed) (Variables|Default|GetMaxSpinSpeed))
            (Variables|Default|SetSpinSpeed (Variables|Default|GetMaxSpinSpeed))))))))

(fn ConstructionScript)

(fn ReverseSpin
  (Variables|Default|SetbSpinReversed (not (Variables|Default|GetbSpinReversed))))