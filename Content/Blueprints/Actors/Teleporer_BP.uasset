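; Paired teleporter actor that sends an overlapping BP_LifeCharacter to its linked OtherTeleporter.
; The sender freezes movement and capsule physics; the receiver moves the character to its spawn actor, sets its own gravity direction on the character and restores physics.
; Timers on the receiver delay re-teleporting to prevent bounce-back and re-enable movement on the player's controlled pawn, and are cleared on EndPlay.
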(event OnComponentBeginOverlap(Box)
  (params (OverlappedComponent :type Primitive%20Component%20Object%20Reference) (OtherActor :type Actor%20Object%20Reference) (OtherComp :type Primitive%20Component%20Object%20Reference) (OtherBodyIndex :type Integer) (bFromSweep :type Boolean) (SweepResult :type Hit%20Result%20Structure%20%28by%20ref%29))
  (bind _asbp_life_character (Utilities|Casting|CastToBP_LifeCharacter OtherActor))
  (CallFunction|DoTeleport _asbp_life_character))

(event EventEndPlay
  (params (EndPlayReason :type EEndPlayReason%20Enum :default "Destroyed"))
  (Utilities|Time|ClearandInvalidateTimerbyHandle (Variables|Default|GetCanMoveTimerHandle))
  (Utilities|Time|ClearandInvalidateTimerbyHandle (Variables|Default|GetCanTeleportTimerHandle)))

(fn ConstructionScript)

(fn DoTeleport
  (params (LifeCharacter :type BP%20Life%20Character%20Object%20Reference))
  (if (Variables|Default|GetCanTeleport)
    (bind _otherteleporter (Variables|Default|GetOtherTeleporter)
      (:then
        (Components|Activation|Activate (Variables|Default|GetTeleportPS) false)
        (Variables|/Game/Blueprints/Pawns/BP_LifeCharacter.BP_LifeCharacter_C|SetCanMove LifeCharacter false)
        (Physics|SetSimulatePhysics (Actor|GetComponentbyClass LifeCharacter "/Script/Engine.CapsuleComponent") false)
        (CallFunction|ReceiveTeleport _otherteleporter LifeCharacter))
      (:else))))

(fn ReceiveTeleport
  (params (LifeCharacter :type BP%20Life%20Character%20Object%20Reference))
  (bind _movementcomponent (Variables|/Script/CustomGravityPlugin.GravityPawn|GetMovementComponent LifeCharacter))
  (Variables|Default|SetCanTeleport false)
  (Variables|/Script/CustomGravityPlugin.GravityMovementComponent|SetSurfaceBasedGravityInfo _movementcomponent (Utilities|Struct|MakeGravityInfo (.GravityPower (Utilities|Struct|BreakGravityInfo (Variables|/Script/CustomGravityPlugin.GravityMovementComponent|GetSurfaceBasedGravityInfo _movementcomponent))) (Variables|Default|GetGravityDirection) (.ForceMode (Utilities|Struct|BreakGravityInfo (Variables|/Script/CustomGravityPlugin.GravityMovementComponent|GetSurfaceBasedGravityInfo _movementcomponent))) (.bForceSubStepping (Utilities|Struct|BreakGravityInfo (Variables|/Script/CustomGravityPlugin.GravityMovementComponent|GetSurfaceBasedGravityInfo _movementcomponent)))))
  (Components|Activation|Activate (Variables|Default|GetTeleportPS) false)
  (bind _returnvalue (Utilities|Time|SetTimerbyFunctionName self "SetCanTeleport" 5.0))
  (Variables|Default|SetCanTeleportTimerHandle _returnvalue)
  (bind _returnvalue_2 (Utilities|Time|SetTimerbyFunctionName self "SetCanMove" 1.0))
  (Variables|Default|SetCanMoveTimerHandle _returnvalue_2)
  (Transformation|SetActorLocation LifeCharacter (Transformation|GetActorLocation (Variables|Default|GetSpawnLocationActor)) false true)
  (Physics|SetSimulatePhysics (Actor|GetComponentbyClass LifeCharacter "/Script/Engine.CapsuleComponent") true))

(fn SetCanTeleport
  (Variables|Default|SetCanTeleport true))

(fn SetCanMove
  (bind _asbp_life_character (Utilities|Casting|CastToBP_LifeCharacter (Pawn|GetControlledPawn (Game|GetPlayerController 0))))
  (Variables|/Game/Blueprints/Pawns/BP_LifeCharacter.BP_LifeCharacter_C|SetCanMove _asbp_life_character true))