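; Spinning fan actor that blows BP_LifeCharacter along world X and fails the level on contact with its box.
; ReverseSpin flips direction, and Tick ramps the yaw spin toward the new maximum speed.
; While a character overlaps the capsule, Tick applies distance-weakened wind force, signed by SpinReversed, unless an X-aligned visibility trace is blocked.
; Box overlap plays a sound and schedules PC_Game's failed-level UI.
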(event OnComponentBeginOverlap(Capsule)
  (params (OverlappedComponent :type Primitive%20Component%20Object%20Reference) (OtherActor :type Actor%20Object%20Reference) (OtherComp :type Primitive%20Component%20Object%20Reference) (OtherBodyIndex :type Integer) (bFromSweep :type Boolean) (SweepResult :type Hit%20Result%20Structure%20%28by%20ref%29))
  (bind _asbp_life_character (Utilities|Casting|CastToBP_LifeCharacter OtherActor))
  (Variables|Default|SetAffectedLifeCharacter _asbp_life_character))

(event OnComponentEndOverlap(Capsule)
  (params (OverlappedComponent :type Primitive%20Component%20Object%20Reference) (OtherActor :type Actor%20Object%20Reference) (OtherComp :type Primitive%20Component%20Object%20Reference) (OtherBodyIndex :type Integer))
  (Utilities|Casting|CastToBP_LifeCharacter OtherActor)
  (Variables|Default|SetAffectedLifeCharacter 0))

(event OnComponentBeginOverlap(Box)
  (params (OverlappedComponent :type Primitive%20Component%20Object%20Reference) (OtherActor :type Actor%20Object%20Reference) (OtherComp :type Primitive%20Component%20Object%20Reference) (OtherBodyIndex :type Integer) (bFromSweep :type Boolean) (SweepResult :type Hit%20Result%20Structure%20%28by%20ref%29))
  (bind _asbp_life_character (Utilities|Casting|CastToBP_LifeCharacter OtherActor))
  (if (Utilities|IsValid (Game|GetInstigatorController _asbp_life_character))
    (bind _aspc_game (Utilities|Casting|CastToPC_Game (Game|GetInstigatorController _asbp_life_character)))
    (Utilities|Time|SetTimerbyFunctionName _aspc_game "ShowFailedLevelUI" 1.0)
    (Audio|PlaySound2D "/Game/Assets/Sounds/raw/felloutofworld.felloutofworld" 1.0 1.0 0.0 0 0)))

(event EventBeginPlay
  (if (Variables|Default|GetbSpinReversed)
    (Variables|Default|SetSpinSpeed (* -1 (Variables|Default|GetMaxSpinSpeed)))
    (else
      (Variables|Default|SetSpinSpeed (Variables|Default|GetMaxSpinSpeed)))))

(event EventTick
  (params (DeltaSeconds :type Float%20%28single-precision%29))
  (Utilities|FlowControl|Sequence
    (:then_0
      (Transformation|AddRelativeRotation (Variables|Default|GetScene) (Math|Rotator|MakeRotator 0.0 0.0 (* (Variables|Default|GetSpinSpeed) DeltaSeconds)) false false))
    (:then_1
      (if (Variables|Default|GetbSpinReversed)
        (Variables|Default|SetSpinSpeed (- (Variables|Default|GetSpinSpeed) (Variables|Default|GetSpeedChange)))
        (if (< (Variables|Default|GetSpinSpeed) (* -1 (Variables|Default|GetMaxSpinSpeed)))
          (Variables|Default|SetSpinSpeed (* -1 (Variables|Default|GetMaxSpinSpeed))))
        (else
          (Variables|Default|SetSpinSpeed (+ (Variables|Default|GetSpinSpeed) (Variables|Default|GetSpeedChange)))
          (if (> (Variables|Default|GetSpinSpeed) (Variables|Default|GetMaxSpinSpeed))
            (Variables|Default|SetSpinSpeed (Variables|Default|GetMaxSpinSpeed))))))
    (:then_2
      (bind _affectedlifecharacter (Variables|Default|GetAffectedLifeCharacter)
        (:then
          (bind _outhit (Collision|LineTraceByChannel (Transformation|GetActorLocation _affectedlifecharacter) (Math|Vector|MakeVector (.X (Math|Vector|BreakVector (Transformation|GetWorldLocation (Variables|Default|GetScene)))) (.Y (Math|Vector|BreakVector (Transformation|GetActorLocation _affectedlifecharacter))) (.Z (Math|Vector|BreakVector (Transformation|GetActorLocation _affectedlifecharacter)))) "TraceTypeQuery1" false 0 "ForOneFrame"))
          (if (not (.bBlockingHit (Collision|BreakHitResult _outhit)))
            (if (Variables|Default|GetbSpinReversed)
              (Class|GravityPawn|AddExternalForce _affectedlifecharacter (* (* (Math|Vector|MakeVector (Math|Float|Absolute(Float) (.X (Math|Vector|BreakVector (Math|Vector|Normalize (- (Transformation|GetActorLocation _affectedlifecharacter) (Math|Vector|MakeVector (.X (Math|Vector|BreakVector (Transformation|GetWorldLocation (Variables|Default|GetScene)))) (.Y (Math|Vector|BreakVector (Transformation|GetActorLocation _affectedlifecharacter))) (.Z (Math|Vector|BreakVector (Transformation|GetActorLocation _affectedlifecharacter))))))))) 0.0 0.0) (/ (* DeltaSeconds (Variables|Default|GetWindForce)) (/ (Math|Vector|VectorLength (- (Transformation|GetActorLocation _affectedlifecharacter) (Math|Vector|MakeVector (.X (Math|Vector|BreakVector (Transformation|GetWorldLocation (Variables|Default|GetScene)))) (.Y (Math|Vector|BreakVector (Transformation|GetActorLocation _affectedlifecharacter))) (.Z (Math|Vector|BreakVector (Transformation|GetActorLocation _affectedlifecharacter)))))) 5e+02))) 1e+05))
              (else
                (Class|GravityPawn|AddExternalForce _affectedlifecharacter (* (* (Math|Vector|MakeVector (Math|Float|Absolute(Float) (.X (Math|Vector|BreakVector (Math|Vector|Normalize (- (Transformation|GetActorLocation _affectedlifecharacter) (Math|Vector|MakeVector (.X (Math|Vector|BreakVector (Transformation|GetWorldLocation (Variables|Default|GetScene)))) (.Y (Math|Vector|BreakVector (Transformation|GetActorLocation _affectedlifecharacter))) (.Z (Math|Vector|BreakVector (Transformation|GetActorLocation _affectedlifecharacter))))))))) 0.0 0.0) (/ (* DeltaSeconds (Variables|Default|GetWindForce)) (/ (Math|Vector|VectorLength (- (Transformation|GetActorLocation _affectedlifecharacter) (Math|Vector|MakeVector (.X (Math|Vector|BreakVector (Transformation|GetWorldLocation (Variables|Default|GetScene)))) (.Y (Math|Vector|BreakVector (Transformation|GetActorLocation _affectedlifecharacter))) (.Z (Math|Vector|BreakVector (Transformation|GetActorLocation _affectedlifecharacter)))))) 5e+02))) -1e+05))))))
        (:else)))))

(fn ConstructionScript)

(fn ReverseSpin
  (Variables|Default|SetbSpinReversed (not (Variables|Default|GetbSpinReversed))))