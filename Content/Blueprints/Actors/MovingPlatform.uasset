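; Moving platform actor that shuttles continuously between the transforms of two referenced actors, Start and End.
; On BeginPlay it snaps to the Start location and plays MoveTimeline, whose Alpha lerps location and rotation each update without sweeping.
; When the timeline finishes, its direction decides whether it reverses or plays from start, creating an endless ping-pong.
; MovePlatformFromStart also exposes a plain Play call on the timeline.
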(event EventBeginPlay
  (bind _movetimeline (Variables|Default|GetMoveTimeline))
  (Utilities|FlowControl|Sequence
    (:then_0
      (Transformation|SetActorLocation (Transformation|GetActorLocation (Variables|Default|GetStart)) false false))
    (:then_1
      (bind (_direction _alpha) (Timeline|MoveTimeline Play)
        (:Update
          (Transformation|SetActorLocation (Math|Vector|Lerp(Vector) (Transformation|GetActorLocation (Variables|Default|GetStart)) (Transformation|GetActorLocation (Variables|Default|GetEnd)) _alpha) false false)
          (Transformation|SetActorRotation (Math|Rotator|Lerp(Rotator) (Transformation|GetActorRotation (Variables|Default|GetStart)) (Transformation|GetActorRotation (Variables|Default|GetEnd)) _alpha)))
        (:Finished
          (if (Utilities|Enum|Equal(Enum) _direction "Backward")
            (Components|Timeline|PlayfromStart _movetimeline)
            (else
              (Utilities|String|Reverse _movetimeline))))))))

(fn ConstructionScript)

(fn MovePlatformfromStart
  (Audio|Components|Audio|Play (Variables|Default|GetMoveTimeline)))