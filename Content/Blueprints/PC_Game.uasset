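; Player controller that runs the HUD, pause input, level music and end-of-level screens.
; On BeginPlay it creates the HUD and loads or creates the LifeSaveGame.
; Finishing a level shows the win UI after a timer, switches to a finish camera, saves completion and picked-up coins per level, and flags game completion from the coin total.
; Failure shows its own UI and camera switch without saving.
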(event EventBeginPlay
  (bind _self self)
  (Utilities|FlowControl|Sequence
    (:then_0
      (bind _returnvalue (UserInterface|CreateWidget "/Game/Blueprints/UMG/HUD.HUD_C" _self _self))
      (bind _output_get (Variables|Default|SetHUD_UI _returnvalue))
      (UserInterface|Viewport|AddtoPlayerScreen _output_get)
      (Input|SetInputModeGameOnly self)
      (Input|EnableInput self))
    (:then_1
      (CallFunction|GetSaveGameData))))

(event EventOnFinishLevel
  (Utilities|Time|SetTimerbyFunctionName 0 "ShowFinishLevelUI" 1.5))

(event Input|ActionEvents|InputActionQuitPause
  (params (Key :type Key%20Structure))
  (:Pressed
    (bind _returnvalue (Game|SetGamePaused (Variables|Default|GetbIsPaused)))
    (Variables|Default|SetbIsPaused _returnvalue)))

(fn ConstructionScript)

(fn ShowFinishLevelUI
  (bind _lifesavegameinstance (Variables|Default|GetLifeSaveGameInstance))
  (bind _lifesavegameinstance_2 (Variables|Default|GetLifeSaveGameInstance))
  (bind _lifesavegameinstance_3 (Variables|Default|GetLifeSaveGameInstance))
  (bind _lifesavegameinstance_4 (Variables|Default|GetLifeSaveGameInstance))
  (bind _lifesavegameinstance_5 (Variables|Default|GetLifeSaveGameInstance))
  (bind _lifesavegameinstance_6 (Variables|Default|GetLifeSaveGameInstance))
  (Utilities|FlowControl|Sequence
    (:then_0
      (Audio|PlaySound2D "/Game/Assets/Sounds/level_win.level_win" 1.0 1.0 0.0 0 0)
      (CallFunction|StopLevelMusic)
      (Variables|Default|SetbShowMouseCursor self true)
      (Widget|RemovefromParent (Variables|Default|GetHUD_UI))
      (bind _returnvalue (UserInterface|CreateWidget "/Game/Blueprints/UMG/FinishedLevel_UI.FinishedLevel_UI_C"))
      (UserInterface|Viewport|AddtoPlayerScreen _returnvalue)
      (Input|SetInputModeUIOnly self 0 "DoNotLock"))
    (:then_1
      (bind _outactors (Actor|GetAllActorsOfClass "/Game/Blueprints/Actors/FinishedCameraActor.FinishedCameraActor_C"))
      (for _array_element _outactors
        (Class|LifePlayerController|SwitchtoExternalCamera _array_element)))
    (:then_3
      (switch int (Variables|Default|GetCurrentLevel)
        (:1
          ;[1 1 1] Level 1 save data
          (Utilities|Array|AddUnique (Variables|/Game/Blueprints/LifeSaveGame.LifeSaveGame_C|GetCompletedLevels _lifesavegameinstance_2) (Variables|Default|GetCurrentLevel))
          (bind _aspc_game (Utilities|Casting|CastToPC_Game (Game|GetPlayerController 0)))
          (for _array_element_2 (Variables|/Script/Life.LifePlayerController|GetPickedUpCoins _aspc_game)
            (Utilities|Array|AddUnique (Variables|/Game/Blueprints/LifeSaveGame.LifeSaveGame_C|GetLevel1Coins _lifesavegameinstance_2) (Variables|/Script/Life.LifePickup_Coin|GetCoinIndex _array_element_2))))
        (:2
          ;[1 1 1] Level 2 save data
          (Utilities|Array|AddUnique (Variables|/Game/Blueprints/LifeSaveGame.LifeSaveGame_C|GetCompletedLevels _lifesavegameinstance_3) (Variables|Default|GetCurrentLevel))
          (bind _aspc_game_2 (Utilities|Casting|CastToPC_Game (Game|GetPlayerController 0)))
          (for _array_element_3 (Variables|/Script/Life.LifePlayerController|GetPickedUpCoins _aspc_game_2)
            (Utilities|Array|AddUnique (Variables|/Game/Blueprints/LifeSaveGame.LifeSaveGame_C|GetLevel2Coins _lifesavegameinstance_3) (Variables|/Script/Life.LifePickup_Coin|GetCoinIndex _array_element_3))))
        (:3
          ;[1 1 1] Level 3 save data
          (Utilities|Array|AddUnique (Variables|/Game/Blueprints/LifeSaveGame.LifeSaveGame_C|GetCompletedLevels _lifesavegameinstance_4) (Variables|Default|GetCurrentLevel))
          (bind _aspc_game_3 (Utilities|Casting|CastToPC_Game (Game|GetPlayerController 0)))
          (for _array_element_4 (Variables|/Script/Life.LifePlayerController|GetPickedUpCoins _aspc_game_3)
            (Utilities|Array|AddUnique (Variables|/Game/Blueprints/LifeSaveGame.LifeSaveGame_C|GetLevel3Coins _lifesavegameinstance_4) (Variables|/Script/Life.LifePickup_Coin|GetCoinIndex _array_element_4))))
        (:4
          ;[1 1 1] Level 4 save data
          (Utilities|Array|AddUnique (Variables|/Game/Blueprints/LifeSaveGame.LifeSaveGame_C|GetCompletedLevels _lifesavegameinstance_6) (Variables|Default|GetCurrentLevel))
          (bind _aspc_game_4 (Utilities|Casting|CastToPC_Game (Game|GetPlayerController 0)))
          (for _array_element_5 (Variables|/Script/Life.LifePlayerController|GetPickedUpCoins _aspc_game_4)
            (Utilities|Array|AddUnique (Variables|/Game/Blueprints/LifeSaveGame.LifeSaveGame_C|GetLevel4Coins _lifesavegameinstance_6) (Variables|/Script/Life.LifePickup_Coin|GetCoinIndex _array_element_5))))))
    (:then_4
      ;[1 1 1] Save the game
      (Utilities|FlowControl|Sequence
        (:then_0
          (Variables|Default|SetbGotAllCoins (== (+ (+ (+ (Utilities|Array|Length (Variables|/Game/Blueprints/LifeSaveGame.LifeSaveGame_C|GetLevel1Coins _lifesavegameinstance)) (Utilities|Array|Length (Variables|/Game/Blueprints/LifeSaveGame.LifeSaveGame_C|GetLevel2Coins _lifesavegameinstance))) (Utilities|Array|Length (Variables|/Game/Blueprints/LifeSaveGame.LifeSaveGame_C|GetLevel3Coins _lifesavegameinstance))) (Utilities|Array|Length (Variables|/Game/Blueprints/LifeSaveGame.LifeSaveGame_C|GetLevel4Coins _lifesavegameinstance))) 5)))
        (:then_1
          (Variables|/Game/Blueprints/LifeSaveGame.LifeSaveGame_C|SetCompletedGame (Variables|Default|GetLifeSaveGameInstance) (Variables|Default|GetbGotAllCoins))
          (SaveGame|SaveGametoSlot _lifesavegameinstance_5 (Variables|/Game/Blueprints/LifeSaveGame.LifeSaveGame_C|GetSaveGameName _lifesavegameinstance_5) (Variables|/Game/Blueprints/LifeSaveGame.LifeSaveGame_C|GetSaveUserIndex _lifesavegameinstance_5)))))))

(fn ShowFailedLevelUI
  (Utilities|FlowControl|Sequence
    (:then_0
      (Audio|PlaySound2D "/Game/Assets/Sounds/level_fail.level_fail" 1.0 1.0 0.0 0 0)
      (CallFunction|StopLevelMusic)
      (Variables|Default|SetbShowMouseCursor self true)
      (Widget|RemovefromParent (Variables|Default|GetHUD_UI))
      (bind _returnvalue (UserInterface|CreateWidget "/Game/Blueprints/UMG/FailedLevel_UI.FailedLevel_UI_C"))
      (UserInterface|Viewport|AddtoPlayerScreen _returnvalue)
      (Input|SetInputModeUIOnly self 0 "DoNotLock"))
    (:then_1
      (bind _outactors (Actor|GetAllActorsOfClass "/Game/Blueprints/Actors/FinishedCameraActor.FinishedCameraActor_C"))
      (for _array_element _outactors
        (Class|LifePlayerController|SwitchtoExternalCamera _array_element)))))

(fn PlayLevelMusic
  (params (SoundCue :type Sound%20Cue%20Object%20Reference))
  (bind _returnvalue (Audio|SpawnSound2D self SoundCue 1.0 1.0 0.0 0))
  (Variables|Default|SetLevelMusic _returnvalue))

(fn StopLevelMusic
  (bind _levelmusic (Variables|Default|GetLevelMusic)
    (:then
      (Audio|Components|Audio|Stop _levelmusic))
    (:else)))

(fn GetSaveGameData
  (Variables|Default|GetLifeSaveGameInstance
    (:then)
    (:else
      (bind _returnvalue (SaveGame|CreateSaveGameObject "/Game/Blueprints/LifeSaveGame.LifeSaveGame_C"))
      (bind _output_get (Variables|Default|SetLifeSaveGameInstance _returnvalue))
      (bind _returnvalue_2 (SaveGame|LoadGamefromSlot (Variables|/Game/Blueprints/LifeSaveGame.LifeSaveGame_C|GetSaveGameName _output_get) (Variables|/Game/Blueprints/LifeSaveGame.LifeSaveGame_C|GetSaveUserIndex _output_get)))
      (bind _aslife_save_game (Utilities|Casting|CastToLifeSaveGame _returnvalue_2))
      (Variables|Default|SetLifeSaveGameInstance _aslife_save_game))))