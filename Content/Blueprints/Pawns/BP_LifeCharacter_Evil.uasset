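; BP_LifeCharacter_Evil is a character Blueprint, apparently an evil variant of LifeCharacter, with helpers for planet-based gravity.
; GetClosestPlanet scans every PlanetActor_BP and keeps the nearest in ClosestPlanet.
; SetSurfacePhysics switches player pawn 0, rather than itself, to surface-normal standing and falling orientation with default gravity.
; SetPointPhysics and the construction script are empty, and nothing here calls the helpers.
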(fn ConstructionScript)

(fn SetPointPhysics)

(fn SetSurfacePhysics
  (bind _aslife_character (Utilities|Casting|CastToLifeCharacter (Game|Player|GetPlayerPawn 0)))
  (Variables|/Script/CustomGravityPlugin.GravityMovementComponent|SetStandingVerticalOrientation (Variables|/Script/CustomGravityPlugin.GravityPawn|GetMovementComponent _aslife_character) "EVO_SurfaceNormal")
  (Variables|/Script/CustomGravityPlugin.GravityMovementComponent|SetFallingVerticalOrientation (Variables|/Script/CustomGravityPlugin.GravityPawn|GetMovementComponent _aslife_character) "EVO_SurfaceNormal")
  (Variables|/Script/CustomGravityPlugin.GravityMovementComponent|SetCustomGravityType (Variables|/Script/CustomGravityPlugin.GravityPawn|GetMovementComponent _aslife_character) "EGT_Default"))

(fn GetClosestPlanet
  (bind _outactors (Actor|GetAllActorsOfClass "/Game/Blueprints/Actors/PlanetActor_BP.PlanetActor_BP_C"))
  (for _array_element _outactors
    (bind _closest_planet (Variables|Default|GetClosest%20Planet)
      (:then
        (if (> (Transformation|GetDistanceTo _closest_planet) (Transformation|GetDistanceTo _array_element))
          (Variables|Default|SetClosest%20Planet _array_element)))
      (:else
        (Variables|Default|SetClosest%20Planet _array_element))))
  (return (Variables|Default|GetClosest%20Planet)))