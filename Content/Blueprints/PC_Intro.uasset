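; PC_Intro is the player controller for the intro, letting the player leave for the menu with the QuitPause input.
; BeginPlay enables input, and QuitPause opens the Entry level with the menu GameMode passed as a URL option in the level name.
; CreateIntroUI, not called within this Blueprint, adds the Intro_UI widget to the player screen, sets game-only input, hides the cursor and returns the widget.
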(event EventBeginPlay
  (Input|EnableInput self))

(event Input|ActionEvents|InputActionQuitPause
  (params (Key :type Key%20Structure))
  (:Pressed
    (Game|OpenLevel(byName) "Entry?game=/Game/Blueprints/GameMode_Menu_BP.GameMode_Menu_BP_C")))

(fn ConstructionScript)

(fn CreateIntroUI
  (bind _returnvalue (UserInterface|CreateWidget "/Game/Blueprints/UMG/Intro_UI.Intro_UI_C"))
  (bind _output_get (Variables|Default|SetIntroUI _returnvalue))
  (UserInterface|Viewport|AddtoPlayerScreen _output_get)
  (Input|SetInputModeGameOnly self)
  (Variables|Default|SetbShowMouseCursor false)
  (return _output_get))